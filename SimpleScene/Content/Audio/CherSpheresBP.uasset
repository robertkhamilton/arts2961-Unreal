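; An actor that visualizes a sound by scaling two spheres with the perceived loudness of audio channels 0 and 1.
; Construction takes the sound and its duration from the LoudnessAnalyzer and assigns the sound to the Audio component.
; Each playback percent update converts to seconds and samples the analyzer's normalized channel loudness, avoiding Tick.
; PlaySound and StopSound control playback, which BeginPlay does not start.
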(event `self.ReceiveBeginPlay`
  ;[1 1 1] Binds an event to tick (fires every time Audio Playback Percent is updated)
  (add `AudioComponent.OnAudioPlaybackPercent` (`self.Audio`) (delegate `PlaybackPercentEvent`)))

(event `PlaybackPercentEvent`
  (params (PlayingSoundWave :type "SoundWave Object Reference") (PlaybackPercent :type "Float (double-precision)"))
  (bind _returnvalue (* PlaybackPercent (`self.Duration`)))
  ;[1 1 1] Change size of Sphere1 dynamically with audio Perceived Loudness
  (`SceneComponent.SetRelativeScale3D` (`self.Sphere 1`) (`KismetMathLibrary.Conv_DoubleToVector` (`LoudnessNRT.GetNormalizedChannelLoudnessAtTime` (`self.LoudnessAnalyzer`) _returnvalue 0)))
  ;[1 1 1] Change size of Sphere2 dynamically with audio Perceived Loudness
  (`SceneComponent.SetRelativeScale3D` (`self.Sphere 2`) (`KismetMathLibrary.Conv_DoubleToVector` (`LoudnessNRT.GetNormalizedChannelLoudnessAtTime` (`self.LoudnessAnalyzer`) _returnvalue 1))))

(fn `playSound`
  (`AudioComponent.Play` (`self.Audio`) 0.0))

(fn `stopSound`
  (`AudioComponent.Stop` (`self.Audio`)))

(fn `UserConstructionScript`
  (bind _sound (`AudioAnalyzerNRT.Sound` (`self.LoudnessAnalyzer`)))
  ;[1 1 1] Assign sound from Loudness Analyzer
  (`AudioComponent.SetSound` (`self.Audio`) _sound)
  ;[1 1 1] Store sound duration
  (set `self.Duration` (`SoundBase.Duration` _sound)))